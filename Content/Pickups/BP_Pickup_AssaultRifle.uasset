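; Assault rifle pickup that grants ammo to the player on overlap.
; The overlap event runs the parent's handling first, then checks that the overlapping actor is player pawn 0.
; It casts that actor to BP_Player and passes the Ammo value to PickupARAmmo.
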(event `self.ReceiveActorBeginOverlap`
  (params (OtherActor :type "Actor Object Reference"))
  (`parent.ReceiveActorBeginOverlap` OtherActor)
  (if (== OtherActor (`GameplayStatics.GetPlayerPawn` 0))
    (bind _asbp_player (cast `/Game/Player/BP_Player` OtherActor))
    (`/Game/Player/BP_Player.PickupARAmmo` _asbp_player (`self.Ammo`))))

(fn `UserConstructionScript`
  (`parent.UserConstructionScript`))