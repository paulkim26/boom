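; BP_Pickup is a pickup actor that spins and bobs while idle and is collected when the player pawn overlaps it.
; BeginPlay sizes the Sphere from PickupRadius and randomizes starting yaw and bob phase.
; Tick rotates the Scene component and offsets it on a sine wave above the root using delta time.
; On pickup it only prints its Label and destroys itself.
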(event `self.ReceiveBeginPlay`
  ;[1 1 1] Set pickup radius
  (`SphereComponent.SetSphereRadius` (`self.Sphere`) (`self.PickupRadius`) true)
  ;[1 1 1] Randomize idle animation
  (set `self.BobPhase` (`KismetMathLibrary.RandomFloatInRange` 0.0 360.0))
  (`SceneComponent.K2_SetWorldRotation` (`self.Scene`) (`KismetMathLibrary.MakeRotator` 0.0 0.0 (`KismetMathLibrary.RandomFloatInRange` 0.0 360.0)) false false))

(event `self.ReceiveActorBeginOverlap`
  (params (OtherActor :type "Actor Object Reference"))
  ;[1 1 1] Picked up by player
  (if (== OtherActor (`GameplayStatics.GetPlayerPawn` 0))
    (`KismetSystemLibrary.PrintString` (`KismetStringLibrary.Concat_StrStr` "Picked up " (`KismetTextLibrary.Conv_TextToString` (`self.Label`))))
    (`self.K2_DestroyActor`)))

(event `self.ReceiveTick`
  (params (DeltaSeconds :type "Float (single-precision)"))
  ;[1 1 1] Idle animation
  (`self.IdleSpin`)
  (`self.IdleBob`))

(fn `IdleBob`
  (bind _output_get (set `self.BobPhase` (mod (+ (* (`GameplayStatics.GetWorldDeltaSeconds`) (`self.BobSpeed`)) (`self.BobPhase`)) 360.0)))
  (`SceneComponent.K2_SetWorldLocation` (`self.Scene`) (+ (`KismetMathLibrary.MakeVector` 0.0 0.0 (* (`KismetMathLibrary.DegSin` _output_get) (`self.BobOffset`))) (`SceneComponent.K2_GetComponentLocation` (`self.DefaultSceneRoot`)) (`self.FloatingHeightMin`)) false false))

(fn `IdleSpin`
  (`SceneComponent.K2_AddWorldRotation` (`self.Scene`) (`KismetMathLibrary.MakeRotator` 0.0 0.0 (* (`GameplayStatics.GetWorldDeltaSeconds`) (`self.RotationSpeed`))) false false))

(fn `UserConstructionScript`)