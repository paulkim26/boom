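; One link in the bear NPC's chained explosion attack, which travels in a straight line as a series of bursts.
; Initialize stores the remaining count and yaw, then spawns a particle burst and a separate hitbox actor while the count is positive.
; After a short delay it spawns and initializes its successor one Length along that yaw with a decremented count, then destroys itself.
; Its own overlap damage logic is disconnected.
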(event `self.ReceiveBeginPlay`
  (`KismetSystemLibrary.Delay` 0.2)
  (`|ExecutionSequence`
    (:`then_0`
      (if (> (`self.Iteration`) 0)
        (`self.SpawnNextAttack`)))
    (:`then_1`
      (`self.K2_DestroyActor`))))

(event `self.ReceiveActorBeginOverlap`
  (params (OtherActor :type "Actor Object Reference")))

(fn `Initialize`
  (params (Iteration :type Integer) (Yaw :type "Float (double-precision)"))
  (bind _output_get (set `self.Iteration` Iteration))
  (set `self.Yaw` Yaw)
  (if (> _output_get 0)
    (`GameplayStatics.SpawnEmitterAtLocation` "/Game/NPC/Bear/P_Bear_Attack_Explosion.P_Bear_Attack_Explosion" (`SceneComponent.K2_GetComponentLocation` (`self.EmitterSpawn`)) (struct) (0.4 0.4 0.1))
    (`|SpawnActorFromClass` "/Game/NPC/Bear/BP_Bear_Attack_Hitbox.BP_Bear_Attack_Hitbox_C" (`KismetMathLibrary.MakeTransform` (`self.K2_GetActorLocation`)) "Undefined" "OverrideRootScale" null null)))

(fn `SpawnNextAttack`
  (bind _returnvalue (`|SpawnActorFromClass` "BP_Bear_Attack_Explosion_C" (`KismetMathLibrary.MakeTransform` (+ (`self.K2_GetActorLocation`) (`KismetMathLibrary.GreaterGreater_VectorRotator` (`KismetMathLibrary.MakeVector` (`self.Length`)) (`KismetMathLibrary.MakeRotator` 0.0 0.0 (`self.Yaw`))))) "Undefined" "OverrideRootScale" null null))
  (`self.Initialize` _returnvalue (- (`self.Iteration`) 1) (`self.Yaw`)))

(fn `UserConstructionScript`)