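; Bear enemy NPC that spawns facing a random yaw, then turns toward and walks after the player until within close range.
; Tick drives steering and a grounded attack cooldown, spawning a hitbox up close or an explosion ahead at longer range, initialized with yaw and iteration count.
; AttackExplosion briefly flags each attack.
; TakeDamage sets Hit and reduces health; death disables capsule collision and Tick destroys the corpse after a delay.
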(event `self.ReceiveBeginPlay`
  ;[1 1 1] Set random initial direction
  (`self.K2_SetActorRotation` (`KismetMathLibrary.MakeRotator` 0.0 0.0 (`KismetMathLibrary.RandomFloatInRange` -180.0 180.0))))

(event `self.ReceiveTick`
  (params (DeltaSeconds :type "Float (single-precision)"))
  (bind _returnvalue (`KismetMathLibrary.Vector_Distance` (`self.K2_GetActorLocation`) (`self.K2_GetActorLocation` (`GameplayStatics.GetPlayerPawn` 0))))
  (if (`self.Alive`)
    (`|ExecutionSequence`
      (:`then_0`
        ;[1 1 1] Check if within attacking range
        (set `self.AttackClose` (< _returnvalue (`self.AttackCloseRange`)))
        ;[1 1 1] Turn to face player
        (`self.TurnToPlayer`)
        (`self.K2_SetActorRotation` (`KismetMathLibrary.MakeRotator` 0.0 0.0 (+ (.yaw (`self.K2_GetActorRotation`)) (`self.TurnRate`))))
        ;[1 1 1] Move towards player
        (if (not (`self.AttackClose`))
          (`self.WalkForward`)))
      (:`then_1`
        (if (< _returnvalue (`self.AttackFarRange`))
          (if (not (`NavMovementComponent.IsFalling` (`self.CharacterMovement`)))
            (bind _output_get (set `self.AttackCooldownStep` (- (`self.AttackCooldownStep`) (`GameplayStatics.GetWorldDeltaSeconds`))))
            (if (< _output_get 0.0)
              (set `self.AttackCooldownStep` (`self.AttackCooldown`))
              (`self.AttackPound`)
              (set `self.AttackExplosion` true)
              (`KismetSystemLibrary.Delay` 0.1)
              (set `self.AttackExplosion` false))))))
    (else
      ;[1 1 1] Destroy corpse after timeout
      (`KismetSystemLibrary.Delay` 10.0)
      (`self.K2_DestroyActor`))))

(fn `AttackPound`
  (if (`self.AttackClose`)
    ;[1 1 1] Close range attack
    (`|SpawnActorFromClass` "/Game/NPC/Bear/BP_Bear_Attack_Hitbox.BP_Bear_Attack_Hitbox_C" (`KismetMathLibrary.MakeTransform` (`self.K2_GetActorLocation`)) "Undefined" "OverrideRootScale" null null)
    (else
      ;[1 1 1] Far range attack
      (bind _returnvalue (`|SpawnActorFromClass` "/Game/NPC/Bear/BP_Bear_Attack_Explosion.BP_Bear_Attack_Explosion_C" (`KismetMathLibrary.MakeTransform` (+ (`self.K2_GetActorLocation`) (`KismetMathLibrary.GreaterGreater_VectorRotator` (`KismetMathLibrary.MakeVector` 450.0) (`KismetMathLibrary.MakeRotator` 0.0 0.0 (.yaw (`self.K2_GetActorRotation`)))))) "Undefined" "OverrideRootScale" null null))
      (`/Game/NPC/Bear/BP_Bear_Attack_Explosion.Initialize` _returnvalue 5 (.yaw (`self.K2_GetActorRotation`))))))

(fn `Die`
  (set `self.Alive` false)
  (`PrimitiveComponent.SetCollisionEnabled` (`self.CapsuleComponent`) "NoCollision"))

(fn `TakeDamage`
  (params (Amount :type "Float (double-precision)"))
  (if (`self.Alive`)
    (set `self.Hit` true)
    (bind _output_get (set `self.Health` (- (`self.Health`) Amount)))
    (if (<= _output_get 0.0)
      (`self.Die`))))

(fn `TurnToPlayer`
  (bind _returnvalue (mod (+ (- (.yaw (`self.K2_GetActorRotation`)) (.yaw (`KismetMathLibrary.FindLookAtRotation` (`self.K2_GetActorLocation`) (`self.K2_GetActorLocation` (`GameplayStatics.GetPlayerPawn` 0))))) 360.0) 360.0))
  (if (`NavMovementComponent.IsFalling` (`self.CharacterMovement`))
    _
    (elif (> _returnvalue 180.0)
      (if (< _returnvalue 355.0)
        (set `self.TurnRate` (`self.TurnSpeed`))
        (else
          (set `self.TurnRate` 0.0 :!label _label)))
      (elif (> _returnvalue 5.0)
        (set `self.TurnRate` (- 0.0 (`self.TurnSpeed`)))
        (else
          (goto _label))))))

(fn `UserConstructionScript`)

(fn `WalkForward`
  (`self.AddMovementInput` (`KismetMathLibrary.GetForwardVector` (`KismetMathLibrary.MakeRotator` 0.0 0.0 (.yaw (`self.GetControlRotation`)))) (`self.WalkSpeed`)))