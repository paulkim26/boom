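; Base friendly NPC that wanders by alternating between standing still and walking with a slight turn.
; Tick runs a two-state timer that flips Phase and rerolls a random duration and turn speed whenever Step runs out.
; While walking, it adds TurnSpeed to actor yaw each frame, unscaled by delta time.
; Movement input follows the control rotation's yaw, flattened to the ground plane, rather than reading actor rotation.
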(event `self.ReceiveTick`
  (params (DeltaSeconds :type "Float (single-precision)"))
  (`|ExecutionSequence`
    (:`then_0`
      (switch `int` (`self.Phase`)
        (:`1`
          (`self.AddDirection` (`self.TurnSpeed`))
          (`self.WalkForward`))))
    (:`then_1`
      (if (> (`self.Step`) 0.0)
        (set `self.Step` (- (`self.Step`) (`GameplayStatics.GetWorldDeltaSeconds`)))
        (else
          (set `self.Phase` (- 1 (`self.Phase`)))
          (set `self.Step` (`KismetMathLibrary.RandomFloatInRange` 1.5 4.0))
          (set `self.TurnSpeed` (`KismetMathLibrary.RandomFloatInRange` -1.0 1.0)))))))

(fn `AddDirection`
  (params (Yaw :type "Float (double-precision)"))
  (`self.SetDirection` (+ (.yaw (`self.K2_GetActorRotation`)) Yaw)))

(fn `SetDirection`
  (params (Yaw :type "Float (double-precision)"))
  (`self.K2_SetActorRotation` (`KismetMathLibrary.MakeRotator` 0.0 0.0 Yaw)))

(fn `UserConstructionScript`)

(fn `WalkForward`
  (`self.AddMovementInput` (`KismetMathLibrary.GetForwardVector` (`KismetMathLibrary.MakeRotator` 0.0 0.0 (.yaw (`self.GetControlRotation`)))) (`self.WalkSpeed`)))