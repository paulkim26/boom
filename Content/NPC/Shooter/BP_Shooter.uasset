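; BP_Shooter is an enemy NPC that attacks the player from within a set radius.
; Each Tick while alive and in range, it turns to face the player and builds a windup timer, then damages BP_Player directly, with no projectile or trace.
; Leaving the radius resets the windup.
; TakeDamage reduces health and calls Die at zero, which stops attacks, disables collision and sets a short lifespan for removal.
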(event `self.ReceiveTick`
  (params (DeltaSeconds :type "Float (single-precision)"))
  (if (`self.Alive`)
    ;[1 1 1] Check if within attack range
    (bind _output_get (set `self.Attack` (<= (`KismetMathLibrary.VSize` (- (`self.K2_GetActorLocation` (`GameplayStatics.GetPlayerPawn` 0)) (`self.K2_GetActorLocation`))) (`self.AttackRadius`))))
    (if _output_get
      ;[1 1 1] Wind up attack
      (bind _output_get_2 (set `self.AttackWindup` (+ (`self.AttackWindup`) (`GameplayStatics.GetWorldDeltaSeconds`))))
      (`self.TurnToPlayer`)
      ;[1 1 1] Inflict damage on player
      (if (>= _output_get_2 (`self.AttackWindupMax`))
        (set `self.AttackWindup` 0.0)
        (bind _asbp_player (cast `/Game/Player/BP_Player` (`GameplayStatics.GetPlayerPawn` 0)))
        (`/Game/Player/BP_Player.TakeDamage` _asbp_player (`self.Damage`)))
      (else
        (set `self.AttackWindup` 0.0)))))

(fn `Die`
  (set `self.Alive` false)
  (`self.SetActorEnableCollision` false)
  (`self.SetLifeSpan` 5.0))

(fn `TakeDamage`
  (params (Damage :type "Float (double-precision)"))
  (if (`self.Alive`)
    (bind _output_get (set `self.Health` (- (`self.Health`) Damage)))
    (if (<= _output_get 0.0)
      (`self.Die`))))

(fn `TurnToPlayer`
  (`self.K2_SetActorRotation` (`KismetMathLibrary.FindLookAtRotation` (`self.K2_GetActorLocation`) (`self.K2_GetActorLocation` (`GameplayStatics.GetPlayerPawn` 0)))))

(fn `UserConstructionScript`)