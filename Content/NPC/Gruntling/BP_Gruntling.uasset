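; BP_Gruntling is a suicide-bomber NPC that wanders until the player comes within range or damages it, then charges and explodes.
; Tick eases walk speed and steers by yaw, using random timed turns when idle and turning toward the player while showing a lit bomb emitter when aggroed.
; Close range after a delay, or zero health, triggers Explode, spawning an effect and attack hitbox before timed corpse removal.
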(event `self.ReceiveBeginPlay`
  (`self.K2_SetActorRotation` (`KismetMathLibrary.MakeRotator` 0.0 0.0 (`KismetMathLibrary.RandomFloatInRange` -180.0 180.0)))
  (bind _returnvalue (`GameplayStatics.SpawnEmitterAttached` "/Game/NPC/Gruntling/EM_Gruntling_Lit.EM_Gruntling_Lit" (`self.Mesh`) "b_MF_Bomb"))
  (bind _output_get (set `self.Emitter` _returnvalue))
  (`SceneComponent.SetVisibility` _output_get false false))

(event `self.ReceiveTick`
  (params (DeltaSeconds :type "Float (single-precision)"))
  (bind _maxspeed (`self.MaxSpeed`))
  (if (`self.Alive`)
    (`|ExecutionSequence`
      (:`then_0`
        ;[1 1 1] Set direction
        (`self.K2_SetActorRotation` (`KismetMathLibrary.MakeRotator` 0.0 0.0 (+ (.yaw (`self.K2_GetActorRotation`)) (`self.TurnSpeed`))))
        (`self.DecrementStep`)
        ;[1 1 1] Ramp up speed to target gradually
        (set `self.WalkSpeed` (+ (`self.WalkSpeed`) (* (- (`self.TargetWalkSpeed`) (`self.WalkSpeed`)) 0.05)))
        ;[1 1 1] Start running if within aggro range
        (if (or (< (`KismetMathLibrary.Vector_Distance` (`self.K2_GetActorLocation`) (`self.K2_GetActorLocation` (`GameplayStatics.GetPlayerPawn` 0))) (`self.AggroRange`)) (`self.Aggro`))
          (set `self.TargetWalkSpeed` _maxspeed)
          (`self.TurnToPlayer`)
          (`SceneComponent.SetVisibility` (`self.Emitter`) true false)
          (else
            (set `self.TargetWalkSpeed` (* _maxspeed 0.4))
            (`SceneComponent.SetVisibility` (`self.Emitter`) false false))))
      (:`then_1`
        ;[1 1 1] Check attack range
        (bind _newparam (`self.DistanceToPlayer`))
        (set `self.AttackClose` (<= _newparam (`self.AttackRange`))))
      (:`then_2`
        (if (`self.AttackClose`)
          (`KismetSystemLibrary.Delay` 1.0)
          (`self.Explode`)
          (else
            (`self.WalkForward`))))
      (:`then_3`
        ;[1 1 1] Register hit animation
        (if (`self.Hit`)
          (`KismetSystemLibrary.Delay` 0.1)
          (set `self.Hit` false)))
      (:`then_4`
        ;[1 1 1] Register attack animation
        (if (`self.Attack`)
          (`KismetSystemLibrary.Delay` 0.1)
          (set `self.Attack` false))))
    (else
      ;[1 1 1] Destroy corpse after timeout
      (`KismetSystemLibrary.Delay` 10.0)
      (`self.K2_DestroyActor`))))

(fn `DecrementStep`
  (bind _output_get (set `self.Step` (- (`self.Step`) (`GameplayStatics.GetWorldDeltaSeconds`))))
  (if (<= _output_get 0.0)
    (`self.SetTurnMode`)))

(fn `DistanceToPlayer`
  (returns (NewParam :type "Float (double-precision)"))
  (return (`KismetMathLibrary.Vector_Distance` (`self.K2_GetActorLocation`) (`self.K2_GetActorLocation` (`GameplayStatics.GetPlayerPawn` 0)))))

(fn `Explode`
  (set `self.Alive` false)
  (`PrimitiveComponent.SetCollisionEnabled` (`self.CapsuleComponent`) "NoCollision")
  (`GameplayStatics.SpawnEmitterAtLocation` "/Game/SciFiWeapDark/FX/Particles/P_Grenade_Explosion_Dark.P_Grenade_Explosion_Dark" (`self.K2_GetActorLocation`) (struct) (0.5 0.5 0.5))
  (`|SpawnActorFromClass` "/Game/NPC/Bear/BP_Bear_Attack_Hitbox.BP_Bear_Attack_Hitbox_C" (`KismetMathLibrary.MakeTransform` (`self.K2_GetActorLocation`)) "Undefined" "OverrideRootScale" null null)
  (`self.Emitter`
    (:`then`
      (`ActorComponent.K2_DestroyComponent` (`self.Emitter`)))
    (:`else`)))

(fn `SetTurnMode`
  (set `self.TurnSpeed` (`KismetMathLibrary.RandomFloatInRange` -0.75 0.75))
  (set `self.Step` (`KismetMathLibrary.RandomFloatInRange` 0.5 3.0)))

(fn `TakeDamage`
  (params (Amount :type "Float (double-precision)"))
  (if (`self.Alive`)
    (set `self.Aggro` true)
    (set `self.Hit` true)
    (bind _output_get (set `self.Health` (- (`self.Health`) Amount)))
    (if (<= _output_get 0.0)
      (`self.Explode`))))

(fn `TurnToPlayer`
  (bind _returnvalue (mod (+ (- (.yaw (`self.K2_GetActorRotation`)) (.yaw (`KismetMathLibrary.FindLookAtRotation` (`self.K2_GetActorLocation`) (`self.K2_GetActorLocation` (`GameplayStatics.GetPlayerPawn` 0))))) 360.0) 360.0))
  (if (not (`NavMovementComponent.IsFalling` (`self.CharacterMovement`)))
    (set `self.TurnSpeed` 2.0)
    (if (> _returnvalue 180.0)
      (if (< _returnvalue 355.0)
        (set `self.TurnSpeed` (`self.TurnSpeed`))
        (else
          (set `self.TurnSpeed` 0.0 :!label _label)))
      (elif (> _returnvalue 5.0)
        (set `self.TurnSpeed` (- 0.0 (`self.TurnSpeed`)))
        (else
          (goto _label))))))

(fn `UserConstructionScript`)

(fn `WalkForward`
  (`self.AddMovementInput` (`KismetMathLibrary.GetForwardVector` (`KismetMathLibrary.MakeRotator` 0.0 0.0 (.yaw (`self.GetControlRotation`)))) (`self.WalkSpeed`)))