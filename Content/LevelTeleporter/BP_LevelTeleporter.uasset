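; Level teleporter actor that opens another level when the player pawn overlaps it while it is active.
; It activates itself on BeginPlay, and the target level comes from its Level variable.
; Activate and Deactivate functions toggle the Active flag together with a Niagara effect, so the visual matches whether the teleporter works.
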(event `self.ReceiveBeginPlay`
  (`self.Activate`))

(event `self.ReceiveActorBeginOverlap`
  (params (OtherActor :type "Actor Object Reference"))
  (if (== OtherActor (`GameplayStatics.GetPlayerPawn` 0))
    (if (`self.Active`)
      (`GameplayStatics.OpenLevel` (`KismetStringLibrary.Conv_StringToName` (`self.Level`))))))

(fn `Activate`
  (set `self.Active` true)
  (`ActorComponent.Activate` (`self.Niagara`) false))

(fn `Deactivate`
  (set `self.Active` false)
  (`ActorComponent.Deactivate` (`self.Niagara`)))

(fn `UserConstructionScript`)