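; First-person player character with movement, aim, a toggleable flashlight, a HUD, and a BP_Weapon attached to the mesh at spawn.
; Tick drives rate-limited automatic fire, using spread line traces from the camera that consume rifle ammo and damage Gruntlings and Bears.
; Health supports healing and post-hit invincibility, and death reloads the level.
; An eight-slot weapon-switching system exists, but its input triggers are disconnected.
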(event `self.ReceiveBeginPlay`
  (`self.FlashlightOff`)
  (bind _returnvalue (`|SpawnActorFromClass` "/Game/Player/BP_Weapon.BP_Weapon_C" (`KismetMathLibrary.MakeTransform` (0.0 0.0 0.0)) "AlwaysSpawn" "OverrideRootScale" null null))
  (bind _output_get (set `self.CurrentWeapon` _returnvalue))
  (`self.K2_AttachToComponent` _output_get (`self.Mesh`) "grip_point" "SnapToTarget" "SnapToTarget" "SnapToTarget" true)
  (`self.InitHUD`))

(event `InputAction|Fire`
  (params (Key :type "Key Structure"))
  (:`Pressed`
    (set `self.FireButtonDown` true))
  (:`Released`
    (set `self.FireButtonDown` false)))

(event `InputAxis|MoveForward`
  (params (AxisValue :type "Float (single-precision)"))
  ;[1 1 1] Movement Controls
  (`self.AddMovementInput` (`self.GetActorForwardVector`) AxisValue))

(event `InputAxis|MoveRight`
  (params (AxisValue :type "Float (single-precision)"))
  ;[1 1 1] Movement Controls
  (`self.AddMovementInput` (`self.GetActorRightVector`) AxisValue))

(event `self.ReceiveTick`
  (params (DeltaSeconds :type "Float (single-precision)"))
  (`self.DecrementInvincibilityCooldown`)
  (if (<= (`self.FiringRateStep`) 0.0)
    (if (and (`self.FireButtonDown`) (> (`self.AssaultRifleAmmo`) 0))
      ;[1 1 1] Fire bullet
      (`self.Shoot`)
      (set `self.Fire` true)
      (`KismetSystemLibrary.Delay` 0.1)
      (set `self.Fire` false))
    (else
      (set `self.FiringRateStep` (- (`self.FiringRateStep`) (`GameplayStatics.GetWorldDeltaSeconds`))))))

(event `InputAction|Jump`
  (params (Key :type "Key Structure"))
  ;[1 1 1] Movement Controls
  (:`Pressed`
    (`self.Jump`))
  (:`Released`
    (`self.StopJumping`)))

(event `InputAxis|LookUp`
  (params (AxisValue :type "Float (single-precision)"))
  ;[1 1 1] Aim Controls
  (`self.AddControllerPitchInput` AxisValue))

(event `InputAxis|LookRight`
  (params (AxisValue :type "Float (single-precision)"))
  ;[1 1 1] Aim Controls
  (`self.AddControllerYawInput` AxisValue))

(event `Key|F`
  (params (Key :type "Key Structure"))
  (:`Pressed`
    (`self.FlashlightToggle`)))

(event `Key|One`
  (params (Key :type "Key Structure"))
  ;[1 1 1] Switch Weapons
)

(event `Key|Two`
  (params (Key :type "Key Structure"))
  ;[1 1 1] Switch Weapons
)

(event `Key|Three`
  (params (Key :type "Key Structure"))
  ;[1 1 1] Switch Weapons
)

(event `Key|Four`
  (params (Key :type "Key Structure"))
  ;[1 1 1] Switch Weapons
)

(event `Key|Five`
  (params (Key :type "Key Structure"))
  ;[1 1 1] Switch Weapons
)

(event `Key|Six`
  (params (Key :type "Key Structure"))
  ;[1 1 1] Switch Weapons
)

(event `Key|Seven`
  (params (Key :type "Key Structure"))
  ;[1 1 1] Switch Weapons
)

(event `Key|Eight`
  (params (Key :type "Key Structure"))
  ;[1 1 1] Switch Weapons
)

(event `Key|Nine`
  (params (Key :type "Key Structure"))
  ;[1 1 1] Switch Weapons
)

(event `Key|Zero`
  (params (Key :type "Key Structure"))
  ;[1 1 1] Switch Weapons
)

(event `Key|MouseScrollDown`
  (params (Key :type "Key Structure"))
  ;[1 1 1] Switch Weapons
)

(event `Key|MouseScrollUp`
  (params (Key :type "Key Structure"))
  ;[1 1 1] Switch Weapons
)

(fn `CalculateBulletEndpoint`
  (params (Origin :type "Vector Structure") (ForwardVector :type "Vector Structure") (Spread :type "Float (double-precision)") (MaxDistance :type "Float (double-precision)"))
  (returns (Start :type "Vector Structure") (End :type "Vector Structure"))
  (bind _returnvalue (- 0.0 Spread))
  (return Origin (+ Origin (`KismetMathLibrary.GreaterGreater_VectorRotator` (`KismetMathLibrary.MakeVector` MaxDistance) (`KismetMathLibrary.MakeRotator` 0.0 (+ (.pitch (`KismetMathLibrary.Conv_VectorToRotator` ForwardVector)) (`KismetMathLibrary.RandomFloatInRange` _returnvalue Spread)) (+ (.yaw (`KismetMathLibrary.Conv_VectorToRotator` ForwardVector)) (`KismetMathLibrary.RandomFloatInRange` _returnvalue Spread)))))))

(fn `DecrementInvincibilityCooldown`
  (if (> (`self.InvincibilityCooldownStep`) 0.0)
    (bind _output_get (set `self.InvincibilityCooldownStep` (- (`self.InvincibilityCooldownStep`) (`GameplayStatics.GetWorldDeltaSeconds`))))
    (if (< _output_get 0.0)
      (set `self.InvincibilityCooldownStep` 0.0))))

(fn `Die`
  (bind _returnvalue (`GameplayStatics.GetCurrentLevelName` true))
  (`GameplayStatics.OpenLevel` (`KismetStringLibrary.Conv_StringToName` _returnvalue)))

(fn `EquipWeapon`
  (bind _returnvalue (`KismetMathLibrary.MakeTransform` (0.0 0.0 0.0)))
  (`/Engine/EditorBlueprintResources/StandardMacros.IsValid` (`self.EquippedGun`)
    (:`Is Valid`
      (`self.K2_DestroyActor` (`self.EquippedGun`)))
    (:`Is Not Valid`
      _))
  (switch `int` (`self.WeaponSlot`)
    (:`Default`
      (`KismetSystemLibrary.PrintString` "Invalid weapon ID"))
    (:`1`
      (bind _returnvalue_2 (`|SpawnActorFromClass` "/Game/Guns/Pistol/BP_Pistol.BP_Pistol_C" _returnvalue "Undefined" "OverrideRootScale" null null))
      (set `self.EquippedGun` _returnvalue_2)
      (`self.K2_AttachToComponent` (`self.EquippedGun`) (`self.GunLocation`) "None" "SnapToTarget" "SnapToTarget" "KeepRelative" true :!label _label))
    (:`2`
      (bind _returnvalue_3 (`|SpawnActorFromClass` "/Game/Guns/AssaultRifle/BP_AssaultRifle.BP_AssaultRifle_C" _returnvalue "Undefined" "OverrideRootScale" null null))
      (set `self.EquippedGun` _returnvalue_3)
      (goto _label))
    (:`3`
      (bind _returnvalue_4 (`|SpawnActorFromClass` "/Game/Guns/Shotgun/BP_Shotgun.BP_Shotgun_C" _returnvalue "Undefined" "OverrideRootScale" null null))
      (set `self.EquippedGun` _returnvalue_4)
      (goto _label))
    (:`4`
      (bind _returnvalue_5 (`|SpawnActorFromClass` "/Game/Guns/Thundergun/BP_Thundergun.BP_Thundergun_C" _returnvalue "Undefined" "OverrideRootScale" null null))
      (set `self.EquippedGun` _returnvalue_5)
      (goto _label))
    (:`5`
      (bind _returnvalue_6 (`|SpawnActorFromClass` "/Game/Guns/Sniper/BP_Sniper.BP_Sniper_C" _returnvalue "Undefined" "OverrideRootScale" null null))
      (set `self.EquippedGun` _returnvalue_6)
      (goto _label))
    (:`6`
      (bind _returnvalue_7 (`|SpawnActorFromClass` "/Game/Guns/Railgun/BP_Railgun.BP_Railgun_C" _returnvalue "Undefined" "OverrideRootScale" null null))
      (set `self.EquippedGun` _returnvalue_7)
      (goto _label))
    (:`7`
      (bind _returnvalue_8 (`|SpawnActorFromClass` "/Game/Guns/GrenadeLauncher/BP_GrenadeLauncher.BP_GrenadeLauncher_C" _returnvalue "Undefined" "OverrideRootScale" null null))
      (set `self.EquippedGun` _returnvalue_8)
      (goto _label))
    (:`8`
      (bind _returnvalue_9 (`|SpawnActorFromClass` "/Game/Guns/RocketLauncher/BP_RocketLauncher2.BP_RocketLauncher2_C" _returnvalue "Undefined" "OverrideRootScale" null null))
      (set `self.EquippedGun` _returnvalue_9)
      (goto _label))))

(fn `FlashlightOff`
  (`SceneComponent.SetVisibility` (`self.Flashlight`) false false))

(fn `FlashlightToggle`
  (`SceneComponent.ToggleVisibility` (`self.Flashlight`) false))

(fn `Heal`
  (params (Amount :type Integer))
  (bind _output_get (set `self.Health` (+ (`self.Health`) Amount)))
  (if (> _output_get 100)
    (set `self.Health` 100)))

(fn `InitHUD`
  (bind _returnvalue (`|CreateWidget` "/Game/Player/HUD/HUD_Player.HUD_Player_C"))
  (bind _output_get (set `self.HUD` _returnvalue))
  (`UserWidget.AddToViewport` _output_get 0))

(fn `NextWeapon`
  (if (< (`self.WeaponSlot`) (`self.WeaponSlotMax`))
    (bind _result (`/Engine/EditorBlueprintResources/StandardMacros.IncrementInt` (`self.WeaponSlot`))
      (:`  `
        (set `self.WeaponSlot` _result)))
    (else
      (set `self.WeaponSlot` (`self.WeaponSlotMin`))))
  (`self.EquipWeapon`))

(fn `PickupARAmmo`
  (params (Amount :type Integer))
  (bind _assaultriflemax (`self.AssaultRifleMax`))
  (bind _output_get (set `self.AssaultRifleAmmo` (+ (`self.AssaultRifleAmmo`) Amount)))
  (if (> _output_get _assaultriflemax)
    (set `self.AssaultRifleAmmo` _assaultriflemax)))

(fn `PreviousWeapon`
  (if (> (`self.WeaponSlot`) (`self.WeaponSlotMin`))
    (bind _result (`/Engine/EditorBlueprintResources/StandardMacros.DecrementInt` (`self.WeaponSlot`))
      (:`  `
        (set `self.WeaponSlot` _result)))
    (else
      (set `self.WeaponSlot` (`self.WeaponSlotMax`))))
  (`self.EquipWeapon`))

(fn `Shoot`
  (bind _fpscamera (`self.FPSCamera`))
  (bind _muzzle (`/Game/Player/BP_Weapon.Muzzle` (`self.CurrentWeapon`)))
  ;[1 1 1] Muzzle Flash
  (`GameplayStatics.SpawnEmitterAtLocation` "/Game/SciFiWeapDark/FX/Particles/P_Pistol_MuzzleFlash_Dark.P_Pistol_MuzzleFlash_Dark" (+ (/ (`self.GetVelocity`) 100.0) (`SceneComponent.K2_GetComponentLocation` _muzzle)) (`SceneComponent.K2_GetComponentRotation` _muzzle))
  ;[1 1 1] Spawn bullet
  (bind (_start _end) (`self.CalculateBulletEndpoint` (`SceneComponent.K2_GetComponentLocation` _fpscamera) (`SceneComponent.GetForwardVector` _fpscamera) (`self.BulletSpread`) (`self.MaxBulletDistance`)))
  (`self.SpawnBullet` _start _end)
  ;[1 1 1] Add delay based on fire rate
  (set `self.FiringRateStep` (`self.FiringRate`))
  (`/Engine/EditorBlueprintResources/StandardMacros.DecrementInt` (`self.AssaultRifleAmmo`)))

(fn `SpawnBullet`
  (params (StartLocation :type "Vector Structure") (EndLocation :type "Vector Structure"))
  (bind _damage (`self.Damage`))
  (bind (_outhit _returnvalue) (`KismetSystemLibrary.LineTraceSingle` StartLocation EndLocation "TraceTypeQuery1"))
  (if _returnvalue
    (bind (_bblockinghit _binitialoverlap _time _distance _location _impactpoint _normal _impactnormal _physmat _hitactor) (`GameplayStatics.BreakHitResult` _outhit))
    (`GameplayStatics.SpawnEmitterAtLocation` "/Game/SciFiWeapDark/FX/Particles/P_Impact_Metal_Medium_Dark.P_Impact_Metal_Medium_Dark" _location)
    (`|ExecutionSequence`
      (:`then_0`
        (bind _returnvalue_2 (`GameplayStatics.GetObjectClass` _hitactor))
        (if (== _returnvalue_2 "/Game/NPC/Gruntling/BP_Gruntling.BP_Gruntling_C")
          (bind _asbp_gruntling (cast `/Game/NPC/Gruntling/BP_Gruntling` _hitactor))
          (`/Game/NPC/Gruntling/BP_Gruntling.TakeDamage` _asbp_gruntling _damage)))
      (:`then_1`
        (if (== _returnvalue_2 "/Game/NPC/Bear/BP_Bear.BP_Bear_C")
          (bind _asbp_bear (cast `/Game/NPC/Bear/BP_Bear` _hitactor))
          (`/Game/NPC/Bear/BP_Bear.TakeDamage` _asbp_bear _damage))))))

(fn `TakeDamage`
  (params (Amount :type Integer))
  ;[1 1 1] Ignore damage if on invincibility cooldown
  (if (not (> (`self.InvincibilityCooldownStep`) 0.0))
    ;[1 1 1] Decrement health
    (bind _output_get (set `self.Health` (- (`self.Health`) Amount)))
    (if (<= _output_get 0)
      (set `self.Health` 0)
      (`self.Die`)
      (else
        ;[1 1 1] Start invincibility sequence
        (set `self.InvincibilityCooldownStep` (`self.InvincibilityCooldownLength`))))))

(fn `UserConstructionScript`)